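; BP_CameraPawn is the pawn that handles mouse selection of tiles in the game.
; On BeginPlay it finds and stores the level's BP_TileManager.
; A left click traces under the cursor, and on a BP_Tile hit it tints the tile green, shows its borders and calls HideBorders on the manager with that tile.
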(event EventBeginPlay
  (bind _outactors (Actor|GetAllActorsOfClass "/Game/Blueprints/BP_TileManager.BP_TileManager_C"))
  (Variables|Default|SetTileManager (Utilities|Array|Get(acopy) _outactors)))

(event Collision|EventActorBeginOverlap
  (params (OtherActor :type Actor%20Object%20Reference)))

(event EventTick
  (params (DeltaSeconds :type Float%20%28single-precision%29)))

(event Input|MouseEvents|LeftMouseButton
  (params (Key :type Key%20Structure))
  (bind _returnvalue (Game|GetPlayerController 0))
  (bind _array (Utilities|Array|MakeArray "ObjectTypeQuery1" "ObjectTypeQuery2" "ObjectTypeQuery4"))
  (bind (_hitresult _returnvalue_2) (Class|PlayerController|GetHitResultUnderCursorforObjects _returnvalue _array true))
  (:Pressed
    (if _returnvalue_2
      (bind _asbp_tile (Utilities|Casting|CastToBP_Tile (.HitActor (Collision|BreakHitResult _hitresult))))
      (Utilities|FlowControl|Sequence
        (:then_0
          (Rendering|Material|SetVectorParameterValueonMaterials (Variables|/Game/Blueprints/BP_Tile.BP_Tile_C|GetTile _asbp_tile) "Color" "0,255.000000, 0"))
        (:then_1
          (Default|SetBordersVisible _asbp_tile))
        (:then_2
          (Class|TileManager|HideBorders (Variables|Default|GetTileManager) _asbp_tile))))))

(fn ConstructionScript)