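; BP_Tile is a tile actor with four border components (left, right, top and bottom) whose visibility can be toggled.
; SetBordersVisible shows all four borders at once, while separate Hide functions hide each side individually.
; The tile runs no logic of its own in BeginPlay, Tick or its construction script, so it only changes when these functions are called.
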(event EventBeginPlay)

(event Collision|EventActorBeginOverlap
  (params (OtherActor :type Actor%20Object%20Reference)))

(event EventTick
  (params (DeltaSeconds :type Float%20%28single-precision%29)))

(fn ConstructionScript)

(fn SetBordersVisible
  (Utilities|FlowControl|Sequence
    (:then_0
      (Rendering|SetVisibility (Variables|Default|GetRightBorder) true false))
    (:then_1
      (Rendering|SetVisibility (Variables|Default|GetTopBorder) true false))
    (:then_2
      (Rendering|SetVisibility (Variables|Default|GetBottomBorder) true false))
    (:then_3
      (Rendering|SetVisibility (Variables|Default|GetLeftBorder) true false))))

(fn HideLeftBorder
  (Rendering|SetVisibility (Variables|Default|GetLeftBorder) false false))

(fn HideRightBorder
  (Rendering|SetVisibility (Variables|Default|GetRightBorder) false false))

(fn HideTopBorder
  (Rendering|SetVisibility (Variables|Default|GetTopBorder) false false))

(fn HideBottomBorder
  (Rendering|SetVisibility (Variables|Default|GetBottomBorder) false false))